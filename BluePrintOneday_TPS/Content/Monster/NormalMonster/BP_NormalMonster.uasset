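; BP_NormalMonster is a monster Blueprint that takes damage and displays its health on an HP bar widget.
; BPStatusComponent handles the damage and supplies the HP percentage.
; BeginPlay pushes the initial percentage to the WBP_HPBar held by the Widget component, and OnDamage forwards damage to the status component, then refreshes the bar the same way.
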(event EventBeginPlay
  (bind _aswbp_hpbar (Utilities|Casting|CastToWBP_HPBar (UserInterface|GetWidget (Variables|Default|GetWidget))))
  (bind _percent (Default|GetHPPercent (Variables|Default|GetBP_StatusComponent)))
  (Default|SetHPPercent _aswbp_hpbar _percent))

(event Collision|EventActorBeginOverlap
  (params (OtherActor :type Actor%20Object%20Reference)))

(event EventTick
  (params (DeltaSeconds :type Float%20%28single-precision%29)))

(fn ConstructionScript)

(fn OnDamage
  (params (Damage :type Integer))
  (Default|OnDamage (Variables|Default|GetBP_StatusComponent) Damage)
  (bind _aswbp_hpbar (Utilities|Casting|CastToWBP_HPBar (UserInterface|GetWidget (Variables|Default|GetWidget))))
  (bind _percent (Default|GetHPPercent (Variables|Default|GetBP_StatusComponent)))
  (Default|SetHPPercent _aswbp_hpbar _percent))