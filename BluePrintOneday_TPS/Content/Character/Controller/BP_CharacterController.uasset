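; Player controller for BP_Character that turns Enhanced Input actions into look, move, attack and skill commands on the pawn.
; On BeginPlay it adds IMC_Character and caches the player 0 pawn as ControlledPawn.
; Movement passes the controller's own forward vector, flattened and normalized, plus its right vector to the pawn.
; Holding skill sets OnSkill and clears IsMove, while releasing it only clears OnSkill.
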(event Input|EnhancedActionEvents|EnhancedInputActionIA_Look
  (params (ActionValue :type Vector%202D%20Structure) (ElapsedSeconds :type Float%20%28double-precision%29) (TriggeredSeconds :type Float%20%28double-precision%29) (InputAction :type Input%20Action%20Object%20Reference :default "/Game/Character/Input/IA_Look.IA_Look"))
  (Default|Look (Variables|Default|GetControlledPawn) ActionValue))

(event Input|EnhancedActionEvents|EnhancedInputActionIA_Move
  (params (ActionValue :type Vector%202D%20Structure) (ElapsedSeconds :type Float%20%28double-precision%29) (TriggeredSeconds :type Float%20%28double-precision%29) (InputAction :type Input%20Action%20Object%20Reference :default "/Game/Character/Input/IA_Move.IA_Move"))
  (bind _returnvalue (Transformation|GetActorForwardVector))
  (bind _returnvalue_2 (Math|Conversions|ToVector2D(Vector) _returnvalue))
  (bind _returnvalue_3 (Math|Vector2D|Normalize2D _returnvalue_2))
  (Default|Move (Variables|Default|GetControlledPawn) ActionValue (Math|Vector|MakeVector (.x _returnvalue_3) (.y _returnvalue_3) 0.0) (Transformation|GetActorRightVector)))

(event Input|EnhancedActionEvents|EnhancedInputActionIA_Attack
  (params (ActionValue :type Boolean) (ElapsedSeconds :type Float%20%28double-precision%29) (TriggeredSeconds :type Float%20%28double-precision%29) (InputAction :type Input%20Action%20Object%20Reference :default "/Game/Character/Input/IA_Attack.IA_Attack"))
  (:Started
    (Default|Attack (Variables|Default|GetControlledPawn))))

(event Input|EnhancedActionEvents|EnhancedInputActionIA_Skill
  (params (ActionValue :type Boolean) (ElapsedSeconds :type Float%20%28double-precision%29) (TriggeredSeconds :type Float%20%28double-precision%29) (InputAction :type Input%20Action%20Object%20Reference :default "/Game/Character/Input/IA_Skill.IA_Skill"))
  (bind _controlledpawn (Variables|Default|GetControlledPawn))
  (:Started
    (Variables|/Game/Character/BP_Character.BP_Character_C|SetOnSkill _controlledpawn true)
    (Variables|/Game/Character/BP_Character.BP_Character_C|SetisMove _controlledpawn false))
  (:Completed
    (Variables|/Game/Character/BP_Character.BP_Character_C|SetOnSkill _controlledpawn false)))

(event EventBeginPlay
  (Input|AddMappingContext (PlayerController|LocalPlayerSubsystems|GetEnhancedInputLocalPlayerSubsystem self) "/Game/Character/Input/IMC_Character.IMC_Character" 0 "(bIgnoreAllPressedKeysUntilRelease=True,bForceImmediately=False,bNotifyUserSettings=False)")
  (bind _asbp_character (Utilities|Casting|CastToBP_Character (Game|Player|GetPlayerPawn 0)))
  (Variables|Default|SetControlledPawn _asbp_character))

(event EventTick
  (params (DeltaSeconds :type Float%20%28single-precision%29)))

(fn ConstructionScript)