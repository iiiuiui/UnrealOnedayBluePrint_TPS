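; Player-style character Blueprint providing look, movement, a four-step attack combo and skill spawning.
; IsMove gates movement and attacks, while Tick enables CanAttack only when AM_Attack is idle, letting Attack cycle AttackCount and play the matching montage section.
; CreateAttackSkill spawns a projectile-style skill at a given bone, aimed forward, with a debug box.
; CreateRSkill spawns BP_RSkill ahead of the character, and EndRSkill flags it as ended.
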(event EventBeginPlay)

(event Collision|EventActorBeginOverlap
  (params (OtherActor :type Actor%20Object%20Reference)))

(event EventTick
  (params (DeltaSeconds :type Float%20%28single-precision%29))
  (Variables|Default|SetCanAttack (not (Animation|Montage|MontageIsPlaying (Components|SkeletalMesh|GetAnimInstance (Variables|Character|GetMesh)) "/Game/Character/Animation/AM_Attack.AM_Attack"))))

(fn ConstructionScript)

(fn Look
  (params (Input :type Vector%202D%20Structure))
  (Pawn|Input|AddControllerYawInput (.x Input))
  (Pawn|Input|AddControllerPitchInput (.y Input)))

(fn Move
  (params (Input :type Vector%202D%20Structure) (ForwardDirection :type Vector) (RightDirection :type Vector))
  (if (not (Variables|Default|GetisMove))
    (return)
    (else
      (Pawn|Input|AddMovementInput ForwardDirection (.x Input) false)
      (Pawn|Input|AddMovementInput RightDirection (.y Input) false))))

(fn Attack
  (if (not (Variables|Default|GetisMove))
    (return)
    (else
      (Utilities|FlowControl|Sequence
        (:then_0
          (if (Variables|Default|GetCanAttack)
            (bind _result (Math|Integer|IncrementInt (Variables|Default|GetAttackCount))
              (:%20%20
                (if (> _result 4)
                  (Variables|Default|SetAttackCount 1))))
            (else
              (return))))
        (:then_1
          (Animation|PlayAnimMontage "/Game/Character/Animation/AM_Attack.AM_Attack" 1.0 (Utilities|String|StringToName (Utilities|String|ToString(Text) (Utilities|Text|FormatText "Attack{0}" (Variables|Default|GetAttackCount))))))))))

(fn CreateAttackSkill
  (params (BoneName :type Name))
  (bind _returnvalue (Game|SpawnActorfromClass "/Game/Character/Skill/BP_AttackSkill.BP_AttackSkill_C" (Transformation|GetBoneTransform (Variables|Character|GetMesh) BoneName "RTS_World") "Undefined" "MultiplyWithRoot" 0 0))
  (Variables|/Game/Character/Skill/BP_AttackSkill.BP_AttackSkill_C|SetCaster _returnvalue self)
  (bind _output_get (Variables|/Game/Character/Skill/BP_AttackSkill.BP_AttackSkill_C|SetDirection _returnvalue (Math|Vector|Normalize (- (+ (* (Transformation|GetActorForwardVector) 3e+03) (Transformation|GetActorLocation)) (Transformation|GetActorLocation _returnvalue)))))
  (Rendering|Debug|DrawDebugBox (+ (+ (Transformation|GetWorldLocation (Variables|Character|GetMesh)) (* _output_get 5e+02)) "0.000000,0.000000,20.000000") "500.000000,50.000000,1.000000" "(R=1.000000,G=0.000000,B=0.059411,A=1.000000)" (Transformation|GetActorRotation) 3.0 3.0))

(fn CreateRSkill
  (bind _returnvalue (Transformation|GetActorTransform))
  (bind _returnvalue_2 (Game|SpawnActorfromClass "/Game/Character/Skill/BP_RSkill.BP_RSkill_C" (Math|Transform|MakeTransform (+ (* (Transformation|GetActorForwardVector) 1e+03) (.location _returnvalue)) (.rotation _returnvalue) "1.000000,1.000000,1.000000") "Undefined" "MultiplyWithRoot" 0 0))
  (Variables|Default|SetRSkill _returnvalue_2))

(fn EndRSkill
  (Variables|/Game/Character/Skill/BP_RSkill.BP_RSkill_C|SetSkillEnd (Variables|Default|GetRSkill) true))