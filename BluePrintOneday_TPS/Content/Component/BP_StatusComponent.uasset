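; Status component that tracks an owner's hit points.
; OnDamage subtracts damage from HP, clamps it at zero, and returns false once HP is depleted, true otherwise.
; GetHPPercent returns current HP divided by MaxHP as a floating-point ratio.
; The component has no active BeginPlay or Tick logic, so HP changes here only through OnDamage calls.
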(event EventBeginPlay)

(event EventTick
  (params (DeltaSeconds :type Float%20%28single-precision%29)))

(fn OnDamage
  (params (Damage :type Integer))
  (bind _output_get (Variables|Default|SetHP (- (Variables|Default|GetHP) Damage)))
  (if (<= _output_get 0)
    (Variables|Default|SetHP 0)
    (return false)
    (else
      (return true))))

(fn GetHPPercent
  (return (/ (Math|Conversions|ToFloat(Integer) (Variables|Default|GetHP)) (Math|Conversions|ToFloat(Integer) (Variables|Default|GetMaxHP)))))